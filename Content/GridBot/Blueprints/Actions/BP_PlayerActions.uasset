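; BP_PlayerActions is the player's mouse input actor for grid tile interaction, tracking the hovered tile and running swappable left and right click actions.
; Each tick it moves the HOVERED state on the Grid to the tile under the cursor.
; Pressing a button executes its action on that tile, and holding it repeats the action whenever the hovered tile changes.
; SetSelectedActions destroys and respawns the action actors, then broadcasts the change.
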(event Custom|OnHoverTileChanged
  (Utilities|FlowControl|Sequence
    (:then_0
      (if (Variables|Default|GetIsLeftMouseDown)
        (Utilities|IsValid (Variables|Default|GetLeftClickAction)
          (:Is%20Valid
            (Default|ExecuteAction (Variables|Default|GetLeftClickAction) (Variables|Default|GetHoveredTile))))))
    (:then_1
      (if (Variables|Default|GetIsRightClickDown)
        (Utilities|IsValid (Variables|Default|GetRightClickAction)
          (:Is%20Valid
            (Default|ExecuteAction (Variables|Default|GetRightClickAction) (Variables|Default|GetHoveredTile))))))))

(event EventBeginPlay
  (bind _returnvalue (Actor|GetActorOfClass "/Script/Gridbot.Grid"))
  (Variables|Default|SetOtherGrid _returnvalue)
  (bind _returnvalue_2 (Actor|GetActorOfClass "/Game/GridBot/Blueprints/Combat/BP_CombatSystem.BP_CombatSystem_C"))
  (Variables|Default|SetCombatSystem _returnvalue_2)
  (Input|EnableInput (Game|GetPlayerController 0)))

(event EventTick
  (params (DeltaSeconds :type Float%20%28single-precision%29))
  (CallFunction|UpdateTileUnderCursor))

(event Input|MouseEvents|LeftMouseButton
  (params (Key :type Key%20Structure :default "None"))
  (:Pressed
    (CallFunction|UpdateTileUnderCursor)
    (Variables|Default|SetIsLeftMouseDown true)
    (Utilities|IsValid (Variables|Default|GetLeftClickAction)
      (:Is%20Valid
        (Default|ExecuteAction (Variables|Default|GetLeftClickAction) (Variables|Default|GetHoveredTile)))))
  (:Released
    (Variables|Default|SetIsLeftMouseDown false)))

(event Input|MouseEvents|RightMouseButton
  (params (Key :type Key%20Structure :default "None"))
  (:Pressed
    (CallFunction|UpdateTileUnderCursor)
    (Variables|Default|SetIsRightClickDown true)
    (Utilities|IsValid (Variables|Default|GetRightClickAction)
      (:Is%20Valid
        (Default|ExecuteAction (Variables|Default|GetRightClickAction) (Variables|Default|GetHoveredTile)))))
  (:Released
    (Variables|Default|SetIsRightClickDown false)))

(fn ConstructionScript)

(fn UpdateTileUnderCursor
  (bind _othergrid (Variables|Default|GetOtherGrid))
  (bind _returnvalue (Class|Grid|GetTileIndexUnderCursor _othergrid))
  (if (!= _returnvalue (Variables|Default|GetHoveredTile))
    (Class|Grid|RemoveStatefromTile (Variables|Default|GetOtherGrid) (Variables|Default|GetHoveredTile) "HOVERED")
    (Variables|Default|SetHoveredTile _returnvalue)
    (Class|Grid|AddStatetoTile (Variables|Default|GetOtherGrid) (Variables|Default|GetHoveredTile) "HOVERED")
    (CallFunction|OnHoverTileChanged)))

(fn SetSelectedActions
  (params (LeftAction :type BP%20Action%20Class%20Reference) (RightAction :type BP%20Action%20Class%20Reference))
  (Utilities|FlowControl|Sequence
    (:then_0
      (Utilities|IsValid (Variables|Default|GetLeftClickAction)
        (:Is%20Valid
          (Actor|DestroyActor (Variables|Default|GetLeftClickAction))
          (Variables|Default|SetLeftClickAction 0))
        (:Is%20Not%20Valid
          _))
      (if (Utilities|IsValidClass LeftAction)
        (bind _returnvalue (Game|SpawnActorfromClass LeftAction (Math|Transform|MakeTransform "0, 0, 0" "0, 0, 0" "1.000000,1.000000,1.000000") "AlwaysSpawn" 0 self 0))
        (Variables|Default|SetLeftClickAction _returnvalue)))
    (:then_1
      (Utilities|IsValid (Variables|Default|GetRightClickAction)
        (:Is%20Valid
          (Actor|DestroyActor (Variables|Default|GetRightClickAction))
          (Variables|Default|SetRightClickAction 0))
        (:Is%20Not%20Valid
          _))
      (if (Utilities|IsValidClass RightAction)
        (bind _returnvalue_2 (Game|SpawnActorfromClass RightAction (Math|Transform|MakeTransform "0, 0, 0" "0, 0, 0" "1.000000,1.000000,1.000000") "AlwaysSpawn" 0 self 0))
        (Variables|Default|SetRightClickAction _returnvalue_2)))
    (:then_2
      (Default|CallOnActionChanged (Variables|Default|GetLeftClickAction) (Variables|Default|GetRightClickAction)))))