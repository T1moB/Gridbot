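; BP_CombatSystem tracks the units in combat and keeps their grid positions in sync with the tile data.
; Adding or removing a unit updates the list, then calls SetUnitOnGrid, with a sentinel index meaning off-grid.
; SetUnitOnGrid clears the old tile if the unit still occupies it and writes the new occupant back into the GridTiles map.
; It then moves the actor to that tile, or far away when none exists.
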(event EventBeginPlay)

(event Collision|EventActorBeginOverlap
  (params (OtherActor :type Actor%20Object%20Reference)))

(event EventTick
  (params (DeltaSeconds :type Float%20%28single-precision%29)))

(fn ConstructionScript)

(fn AddUnitinCombat
  (params (Unit :type RTS%20Ground%20Unit%20Master%20Object%20Reference) (Index :type Int%20Point%20Structure))
  (Utilities|Array|Add (Variables|Default|GetUnitsInCombat) Unit)
  (CallFunction|SetUnitonGrid Unit Index))

(fn RemoveUnitfromCombat
  (params (Unit :type RTS%20Ground%20Unit%20Master%20Object%20Reference))
  (Utilities|Array|RemoveItem (Variables|Default|GetUnitsInCombat) Unit)
  (CallFunction|SetUnitonGrid Unit (Utilities|Struct|MakeIntPoint -999 -999)))

(fn SetUnitonGrid
  (params (Unit :type RTS%20Ground%20Unit%20Master%20Object%20Reference) (Index :type Int%20Point%20Structure))
  (bind _grid (Variables|Default|GetGrid))
  (bind _gridtiles (Variables|/Script/Gridbot.Grid|GetgridTiles _grid))
  (bind (_value _returnvalue) (Utilities|Map|Find _gridtiles Index))
  (Utilities|FlowControl|Sequence
    (:then_0
      (if (!= (Variables|/Game/RTS_Test/Blueprints/Units/RTS_GroundUnitMaster.RTS_GroundUnitMaster_C|GetIndexOnGrid Unit) Index)
        (Utilities|FlowControl|Sequence
          (:then_0
            (bind _output_get (LocalVariables|SetPreviousTile (.Value (Utilities|Map|Find (Variables|/Script/Gridbot.Grid|GetgridTiles (Variables|Default|GetGrid)) (Variables|/Game/RTS_Test/Blueprints/Units/RTS_GroundUnitMaster.RTS_GroundUnitMaster_C|GetIndexOnGrid Unit)))))
            (if (== (Utilities|Struct|BreakS_TileData _output_get) Unit)
              (bind _structout (Utilities|Struct|SetmembersinS_TileData (LocalVariables|GetPreviousTile)))
              (Utilities|Map|Add (Variables|/Script/Gridbot.Grid|GetgridTiles (Variables|Default|GetGrid)) (Utilities|Struct|BreakS_TileData _structout) _structout)))
          (:then_1
            (Variables|/Game/RTS_Test/Blueprints/Units/RTS_GroundUnitMaster.RTS_GroundUnitMaster_C|SetIndexOnGrid Unit Index)
            (if (!= Index (Utilities|Struct|MakeIntPoint -999 -999))
              (bind _structout_2 (Utilities|Struct|SetmembersinS_TileData (.Value (Utilities|Map|Find (Variables|/Script/Gridbot.Grid|GetgridTiles (Variables|Default|GetGrid)) Index)) Unit))
              (Utilities|Map|Add (Variables|/Script/Gridbot.Grid|GetgridTiles (Variables|Default|GetGrid)) (Utilities|Struct|BreakS_TileData _structout_2) _structout_2))))))
    (:then_1
      (Transformation|SetActorLocation Unit (Math|Vector|SelectVector (.location (Utilities|Struct|BreakS_TileData _value)) "-9999.000000,-9999.000000,-9999.000000" _returnvalue) false false))))