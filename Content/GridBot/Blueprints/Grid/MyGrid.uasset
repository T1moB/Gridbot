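; MyGrid is a grid actor that builds a tile grid and can switch it to a tactical view at runtime.
; Its construction script spawns the grid at the actor's location from the tile size, grid size and environment setting, once the visual child actor is valid.
; The ToggleTacticalGrid event flips the tactical state on the GridVisual object.
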(event Custom|ToggleTacticalGrid
  (bind _gridvisual (Variables|Default|GetgridVisual))
  (Class|GridVisual|SetTacticalGrid _gridvisual (not (Variables|/Script/Gridbot.GridVisual|GetisTactical _gridvisual))))

(event EventBeginPlay)

(event Collision|EventActorBeginOverlap
  (params (OtherActor :type Actor%20Object%20Reference)))

(event EventTick
  (params (DeltaSeconds :type Float%20%28single-precision%29)))

(fn ConstructionScript
  (Utilities|IsValid (Variables|/Script/Engine.ChildActorComponent|GetChildActor (Variables|Default|GetGridVisual_ChildActor))
    (:Is%20Valid
      (Class|Grid|SpawnGrid (Transformation|GetActorLocation) (Variables|Default|GettileSize) (Variables|Default|GetgridSize) (Variables|Default|GetuseEnvironment)))))