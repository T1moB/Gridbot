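; Grid pathfinding actor that searches for a path in timed steps rather than all at once.
; FindPathwithDelay analyzes one discovered tile per iteration, looping through a retriggerable delay until the search succeeds or no discovered indexes remain.
; Success passes the generated path to OnPathFound, while an exhausted search still fires it with a placeholder array.
; The tile analysis and path generation logic are defined outside these graphs.
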(event EventBeginPlay)

(event Collision|EventActorBeginOverlap
  (params (OtherActor :type Actor%20Object%20Reference)))

(event EventTick
  (params (DeltaSeconds :type Float%20%28single-precision%29)))

(event EventFindPathwithDelay
  (if (> (Utilities|Array|Length (Variables|Default|GetdiscoverdIndexes)) 0) :!label _label
    (bind _returnvalue (Class|GridPathfinding|AnalyzeNextDiscoverTile))
    (if _returnvalue
      (bind _returnvalue_2 (Class|GridPathfinding|GeneratePath))
      (Default|CallOnPathFound _returnvalue_2)
      (else
        (Utilities|FlowControl|RetriggerableDelay (Variables|Default|GetdelayBetweenIterations))
        (goto _label)))
    (else
      (Default|CallOnPathFound (Utilities|Array|MakeArray "")))))

(fn ConstructionScript)