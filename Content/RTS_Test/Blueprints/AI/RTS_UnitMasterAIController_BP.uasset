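; Master AI controller for RTS ground units, running the player-unit blackboard and base behavior tree.
; On BeginPlay it caches the RTS player controller and game state, then starts the tree.
; It reads the current game speed from the game state and binds to its speed-control dispatcher to keep the local value updated.
; On possession it stores the pawn as a ground unit master reference.
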(event Custom|GetGameSpeed
  (params (GameSpeed :type Float%20%28single-precision%29))
  (Variables|Default|SetGameSpeed GameSpeed))

(event EventBeginPlay
  (Utilities|RefrenceCast)
  (Class|AIController|UseBlackboard "/Game/RTS_Test/Blueprints/AI/BB_PlayerUnit.BB_PlayerUnit")
  (AI|RunBehaviorTree "/Game/RTS_Test/Blueprints/AI/BT_PlayerUnitBase.BT_PlayerUnitBase")
  (bind _gamespeed (Default|GetGameSpeed (Variables|Refrences|GetGameStateRef)))
  (Variables|Default|SetGameSpeed _gamespeed)
  (EventDispatchers|BindEventtoGameSpeedControl (Variables|Refrences|GetGameStateRef) (EventDispatchers|CreateEvent :!event Custom|GetGameSpeed)))

(event EventPossess
  (params (PossessedPawn :type Pawn%20Object%20Reference))
  (Variables|Refrences|SetUnitRef (.AsRTS%20Ground%20Unit%20Master (Utilities|Casting|CastToRTS_GroundUnitMaster PossessedPawn))))

(fn ConstructionScript)