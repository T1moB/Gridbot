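; RTS game state that runs the in-game clock, calendar and adjustable game speed.
; Each tick advances game time by the current speed, derives time and date with month and year rollover, and pushes both to the player controller's HUD.
; When a day passes, it calls a birthday event on every ground unit.
; Speed changes scale the default by a multiplier and broadcast through GameSpeedControl.
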(event EventBeginPlay
  (Utilities|FlowControl|Sequence
    (:then_0
      (Utilities|ReferenceCast))
    (:then_1
      ;[1 1 1] Set default game clock and calender
      (Variables|GameTimeSettings|SetGameTime (+ (Math|Conversions|ToFloat(Integer) (Variables|Clock|GetHours)) (/ (Math|Conversions|ToFloat(Integer) (Variables|Clock|GetMinutes)) 6e+01) (/ (Math|Conversions|ToFloat(Integer) (Variables|Clock|GetSeconds)) 3.6e+03)))
      (Variables|Calender|SetGameDate (Utilities|Array|MakeArray (Variables|Calender|GetDay) (Variables|Calender|GetMonth) (Variables|Calender|GetYear))))
    (:then_2
      ;[1 1 1] Set default game speed
      (Variables|GameTimeSettings|SetGameSpeed (Variables|GameTimeSettings|GetDefaultGameSpeed)))))

(event EventTick
  (params (DeltaSeconds :type Float%20%28single-precision%29))
  ;[1 1 1] Game Clock
  (Variables|GameTimeSettings|SetGameTime (.GameTime (CallFunction|SetGameTime DeltaSeconds (Variables|GameTimeSettings|GetGameSpeed) (Variables|GameTimeSettings|GetGameTime))))
  (Variables|Calender|SetDayCounter (.DayCount (CallFunction|SetGameTime DeltaSeconds (Variables|GameTimeSettings|GetGameSpeed) (Variables|GameTimeSettings|GetGameTime))))
  (CallFunction|SetClock)
  (CallFunction|SetCalender)
  (if (== (.DayCount (CallFunction|SetGameTime DeltaSeconds (Variables|GameTimeSettings|GetGameSpeed) (Variables|GameTimeSettings|GetGameTime))) 1)
    (bind _unitsout (CallFunction|GetAllUnits))
    (for _array_element _unitsout
      (Default|BirthDayEvent _array_element))))

(event EventUpdateGameSpeed
  (params (SpeedMultiplier :type Float%20%28double-precision%29))
  (bind _output_get (Variables|GameTimeSettings|SetSpeedMultiplier SpeedMultiplier))
  (bind _output_get_2 (Variables|GameTimeSettings|SetGameSpeed (* _output_get (Variables|GameTimeSettings|GetDefaultGameSpeed))))
  (Default|CallGameSpeedControl _output_get_2))

(fn ConstructionScript)

(fn SetClock
  (bind _gametime (Variables|GameTimeSettings|GetGameTime))
  (bind _returnvalue (* _gametime 3.6e+03))
  (bind (_remainder _returnvalue_2) (Math|Float|Division(WholeandRemainder) _returnvalue 6e+01))
  (bind _returnvalue_3 (Math|Conversions|ToFloat(Integer) _returnvalue_2))
  (bind (_remainder_2 _returnvalue_4) (Math|Float|Division(WholeandRemainder) _returnvalue_3 6e+01))
  (Variables|Clock|SetSeconds (Math|Float|Floor _remainder))
  (Variables|Clock|SetMinutes (Math|Float|Floor _remainder_2))
  (Variables|Clock|SetHours (Math|Float|Floor (.Remainder (Math|Float|Division(WholeandRemainder) (Math|Conversions|ToFloat(Integer) _returnvalue_4) 24.0))))
  (bind _output_get (Variables|Calender|SetGameDate (Utilities|Array|MakeArray (Variables|Clock|GetSeconds) (Variables|Clock|GetMinutes) (Variables|Clock|GetHours))))
  (Default|SetTime (Variables|/Game/RTS_Test/Blueprints/GameSettings/RTS_PlayerController_BP.RTS_PlayerController_BP_C|GetMainGameHudRef (Variables|References|GetControllerRef)) _output_get))

(fn SetCalender
  (bind _output_get (Variables|Calender|SetDay (+ (Variables|Calender|GetDay) (Variables|Calender|GetDayCounter))))
  (if (> _output_get (Class|KismetMathLibrary|DaysinMonth (Variables|Calender|GetYear) (Variables|Calender|GetMonth)))
    (Variables|Calender|SetDay 1)
    (Variables|Calender|SetMonth (+ (Variables|Calender|GetMonth) 1)))
  (if (> (Variables|Calender|GetMonth) 12)
    (Variables|Calender|SetMonth 1)
    (Variables|Calender|SetYear (+ (Variables|Calender|GetYear) 1)))
  (bind _output_get_2 (Variables|Calender|SetGameDate (Utilities|Array|MakeArray (Variables|Calender|GetDay) (Variables|Calender|GetMonth) (Variables|Calender|GetYear))))
  (Default|SetDate (Variables|/Game/RTS_Test/Blueprints/GameSettings/RTS_PlayerController_BP.RTS_PlayerController_BP_C|GetMainGameHudRef (Variables|References|GetControllerRef)) _output_get_2))

(fn GetGameSpeed
  (return (Variables|GameTimeSettings|GetGameSpeed)))

(fn GetAllUnits
  (bind _outactors (Actor|GetAllActorsOfClass "/Game/RTS_Test/Blueprints/Units/RTS_GroundUnitMaster.RTS_GroundUnitMaster_C"))
  (bind _output_get (Variables|Default|SetListOfAllUnits _outactors))
  (return _output_get))