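; RTS player controller that drives the camera, unit selection and unit orders, spawning the unit trainer and main HUD at startup.
; It moves the camera pawn with keys and edge scrolling, using gated mouse axes for rotation and the spring arm for zoom.
; Left-click feeds marquee selection in the HUD class.
; Right-click issues AI moves to grid-converted locations with decals or infantry attacks on units; debug keys spawn units and change game speed.
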(event Custom|UpdateMarquee
  ;[1 1 1] Marquee Selection
  ;;[1 1 1] Update Mouse Location
  (if (Variables|Marquee|GetIsHoldingInput)
    (Variables|Marquee|SetHoldingTime (+ (Variables|Marquee|GetHoldingTime) (Variables|Marquee|GetDeltaTime)))
    (Class|MarqueeSelectionIF|OnInputHold(Message) (Variables|References|GetMarqueeHudRef))))

(event Custom|RemoveLocationDecal
  (bind _targetlocationdecal (Variables|Default|GetTargetLocationDecal))
  ;[1 1 1] Destroy Movement Decal
  (Utilities|IsValid _targetlocationdecal
    (:Is%20Valid
      (Components|DestroyComponent _targetlocationdecal))))

(event Custom|MoveToUnit
  ;[1 1 1] Unit Movements
  ;;[1 1 1] Move To Unit
  (Default|SetTargetUnit (Variables|Unit|GetSelectedUnit) (Variables|Default|GetTargetUnit))
  (switch Utilities|FlowControl|Switch|SwitchonUnitTypes_ENUM (Variables|/Game/RTS_Test/Blueprints/Units/RTS_GroundUnitMaster.RTS_GroundUnitMaster_C|GetUnitType (Variables|Unit|GetSelectedUnit))
    (:NewEnumerator0
      (Utilities|InfantryAttack
        (:On%20Move%20Finished
          (Default|PreparetoAttack (Variables|Unit|GetSelectedUnit)))))))

(event Custom|StartMarqueeSelect
  ;[1 1 1] Marquee Selection
  ;;[1 1 1] On Left Click
  (Class|MarqueeSelectionIF|OnInputStart(Message) (Variables|References|GetMarqueeHudRef))
  (Variables|Marquee|SetHoldingTime 0.0)
  (Variables|Marquee|SetIsHoldingInput true))

(event Custom|SimpleMoveToLocation
  ;[1 1 1] Unit Movements
  ;;[1 1 1] Move To Location
  (Utilities|MovetoMacro
    (:On%20Move%20Finished
      (CallFunction|RemoveLocationDecal))))

(event EventBeginPlay
  (bind _girdsize (Variables|Grid|GetGirdSize))
  (bind _returnvalue (/ 1.0 _girdsize))
  (Utilities|FlowControl|Sequence
    (:then_0
      (Utilities|ReferenceCast) ; Should always be first
    )
    (:then_1
      (bind _returnvalue_2 (Game|SpawnActorfromClass "/Game/RTS_Test/Blueprints/Units/RTS_UnitTrainer.RTS_UnitTrainer_C" (Variables|Construction|GetEmptyTransform) "AlwaysSpawn" 0 self 0))
      (Variables|References|SetUnitTrainerRef _returnvalue_2))
    (:then_2
      (Utilities|SpawnWidgets)
      (UserInterface|Viewport|AddtoViewport (Variables|References|GetMainGameHudRef) 1)
      (HUD|SetHudVisibility "Visible"))
    (:then_3
      (Input|SetInputModeGameandUI self 0 "DoNotLock" false false))
    (:then_4
      (Variables|Grid|SetGridScale (Math|Vector|MakeVector _returnvalue _returnvalue 0.0)))))

(event EventTick
  (params (DeltaSeconds :type Float%20%28single-precision%29))
  ;[1 1 1] Event Tick (Update)
  (Variables|Marquee|SetDeltaTime DeltaSeconds)
  (if (Variables|Marquee|GetIsHoldingInput)
    (CallFunction|UpdateMarquee)))

(event Input|ActionEvents|InputActionZoomReset
  (params (Key :type Key%20Structure))
  ;[1 1 1] Camera Zoom
  ;;[1 1 1] Zoom Reset
  (:Pressed
    (Variables|/Script/Engine.SpringArmComponent|SetTargetArmLength (Variables|/Game/RTS_Test/Blueprints/GameSettings/CameraPawn_BP.CameraPawn_BP_C|GetSpringArm (Variables|References|GetCameraPawnRef)) (Variables|CameraZoom|GetStartZoom))))

(event Input|ActionEvents|InputActionSecondaryAction
  (params (Key :type Key%20Structure))
  ;[1 1 1] Right Click Commands
  (:Pressed
    (if (Variables|Unit|GetIsUnitSelected)
      (UnitCommands|SetClickedActor)
      (Utilities|FlowControl|Sequence
        (:then_0
          (Utilities|GetUnitDetails)
          (UnitCommands|StopPreviousCommand)
          (Utilities|GetMovementTarget
            (:MoveToUnit
              (CallFunction|MovetoUnit))
            (:MoveToLocation
              (CallFunction|SimpleMovetoLocation)))))
      (else
        (HUD|GetUnitHud)))))

(event Input|ActionEvents|InputActionPrimaryAction
  (params (Key :type Key%20Structure))
  ;[1 1 1] Left Click Commands
  (:Pressed
    (CallFunction|StartMarqueeSelect))
  (:Released
    (Class|MarqueeSelectionIF|OnInputRelease(Message) (Variables|References|GetMarqueeHudRef) (Variables|Marquee|GetHoldingTime))
    (Variables|Marquee|SetIsHoldingInput false)))

(event Input|ActionEvents|InputActionPan
  (params (Key :type Key%20Structure))
  (bind _camerapawnref (Variables|References|GetCameraPawnRef))
  (bind _returnvalue (Transformation|GetActorRotation _camerapawnref))
  (bind (_roll _pitch _yaw) (Math|Rotator|BreakRotator _returnvalue))
  ;[1 1 1] Camera panning
  ;;[1 1 1] Camera turning
  (:Pressed
    (Utilities|FlowControl|Gate true) ; enters at Open
  )
  (:Released
    (Utilities|FlowControl|Gate true) ; enters at Close
  ))

(event Input|ActionEvents|InputActionPanReset
  (params (Key :type Key%20Structure))
  (bind _camerapawnref (Variables|References|GetCameraPawnRef))
  ;[1 1 1] Camera panning
  ;;[1 1 1] Pan Reset
  (:Pressed
    (Transformation|SetActorRotation _camerapawnref (Math|Rotator|MakeRotator (.Roll (Math|Rotator|BreakRotator (Transformation|GetActorRotation _camerapawnref))) 0.0 0.0))))

(event Input|ActionEvents|InputActionPan
  (params (Key :type Key%20Structure))
  (bind _camerapawnref (Variables|References|GetCameraPawnRef))
  (bind _returnvalue (Transformation|GetActorRotation _camerapawnref))
  (bind (_roll _pitch _yaw) (Math|Rotator|BreakRotator _returnvalue))
  ;[1 1 1] Camera panning
  ;;[1 1 1] Camera turning
  (:Pressed
    (Variables|CameraMovement|SetDisableCameraMovement true)
    (Utilities|FlowControl|Gate true) ; enters at Open
  )
  (:Released
    (Variables|CameraMovement|SetDisableCameraMovement false)
    (Utilities|FlowControl|Gate true) ; enters at Close
  ))

(event Input|ActionEvents|InputActionFastCamera
  (params (Key :type Key%20Structure))
  ;[1 1 1] Set Camera Boost
  (:Pressed
    (Variables|CameraMovement|SetMovementSpeedModifier 2.0))
  (:Released
    (Variables|CameraMovement|SetMovementSpeedModifier 1.0)))

(event Input|AxisEvents|InputAxisMoveForward
  (params (AxisValue :type Float%20%28single-precision%29))
  ;[1 1 1] Camera Movement
  (if (not (Variables|CameraMovement|GetDisableCameraMovement))
    (Utilities|CameraMovement AxisValue (stale Input|AxisEvents|InputAxisMoveRight AxisValue))))

(event Input|AxisEvents|InputAxisZoomIn
  (params (AxisValue :type Float%20%28single-precision%29))
  (bind _camerapawnref (Variables|References|GetCameraPawnRef))
  (bind _springarm (Variables|/Game/RTS_Test/Blueprints/GameSettings/CameraPawn_BP.CameraPawn_BP_C|GetSpringArm _camerapawnref))
  ;[1 1 1] Camera Zoom
  ;;[1 1 1] Zoom in and out
  (Variables|/Script/Engine.SpringArmComponent|SetTargetArmLength _springarm (Math|Float|Clamp(Float) (+ (Variables|/Script/Engine.SpringArmComponent|GetTargetArmLength _springarm) (* AxisValue (Variables|CameraZoom|GetZoomSpeed))) (Variables|CameraZoom|GetMinZoomLimit) (Variables|CameraZoom|GetMaxZoomLimit))))

(event Input|AxisEvents|InputAxisMoveRight
  (params (AxisValue :type Float%20%28single-precision%29))
  ;[1 1 1] Camera Movement
  (if (not (Variables|CameraMovement|GetDisableCameraMovement))
    (Utilities|CameraMovement (stale Input|AxisEvents|InputAxisMoveForward AxisValue) AxisValue)))

(event Input|MouseEvents|MouseX
  (params (AxisValue :type Float%20%28single-precision%29))
  (bind _camerapawnref (Variables|References|GetCameraPawnRef))
  (bind _returnvalue (Transformation|GetActorRotation _camerapawnref))
  (bind (_roll _pitch _yaw) (Math|Rotator|BreakRotator _returnvalue))
  ;[1 1 1] Camera panning
  ;;[1 1 1] Camera turning
  (Utilities|FlowControl|Gate true
    (:Exit
      (Transformation|SetActorRotation _camerapawnref (Math|Rotator|MakeRotator _roll _pitch (+ _yaw (* AxisValue (Variables|CameraPan|GetPanSpeed))))))))

(event Input|MouseEvents|MouseY
  (params (AxisValue :type Float%20%28single-precision%29))
  (bind _camerapawnref (Variables|References|GetCameraPawnRef))
  (bind _returnvalue (Transformation|GetActorRotation _camerapawnref))
  (bind (_roll _pitch _yaw) (Math|Rotator|BreakRotator _returnvalue))
  ;[1 1 1] Camera panning
  ;;[1 1 1] Camera turning
  (Utilities|FlowControl|Gate true
    (:Exit
      (Transformation|SetActorRotation _camerapawnref (Math|Rotator|MakeRotator _roll (Math|Float|Clamp(Float) (+ _pitch (* AxisValue (Variables|CameraPan|GetPanSpeed))) -25.0 4e+01) _yaw)))))

(event Input|MouseEvents|MouseX
  (params (AxisValue :type Float%20%28single-precision%29))
  ;[1 1 1] Edge scroll movement
  (if (not (Variables|CameraMovement|GetDisableCameraMovement))
    (bind (_deltaspeedx _deltaspeedy) (Utilities|EdgeScroll))
    (Utilities|CameraMovement _deltaspeedx _deltaspeedy)))

(event Input|MouseEvents|MouseY
  (params (AxisValue :type Float%20%28single-precision%29))
  ;[1 1 1] Edge scroll movement
  (if (not (Variables|CameraMovement|GetDisableCameraMovement))
    (Utilities|EdgeScroll) ; enters at MouseY
  ))

(event Input|KeyboardEvents|End
  (params (Key :type Key%20Structure))
  ;[1 1 1] Debug Cheat Commands Spawn Unit, Vehicle and speed up time
  (:Pressed
    (Class|GameTimeIF|UpdateGameSpeed(Message) (Variables|References|GetGameStateRef) 2.5e-05)))

(event Input|KeyboardEvents|V
  (params (Key :type Key%20Structure))
  (bind _self self)
  (bind _cursorlocationinworld (CallFunction|GetMousePosinWorld _self 1e+04))
  ;[1 1 1] Debug Cheat Commands Spawn Unit, Vehicle and speed up time
  (:Pressed
    (if true
      (Game|SpawnActorfromClass "/Game/RTS_Test/Blueprints/Units/RTS_GroundUnitMaster.RTS_GroundUnitMaster_C" (Math|Transform|MakeTransform (Math|Vector|MakeVector (.x _cursorlocationinworld) (.y _cursorlocationinworld) 1e+02)) "DontSpawnIfColliding" 0 0))))

(event Input|KeyboardEvents|B
  (params (Key :type Key%20Structure))
  ;[1 1 1] Debug Cheat Commands Spawn Unit, Vehicle and speed up time
)

(fn ConstructionScript)

(fn SetHudVisibility
  (params (MainGameHud :type ESlateVisibility%20Enum :default "Visible"))
  (Widget|SetVisibility (Variables|References|GetMainGameHudRef) MainGameHud))

(fn SetSelectedUnits
  (params (SelectedUnits :type Array%20of%20RTS%20Ground%20Unit%20Master%20Object%20References))
  (Variables|Unit|SetSelectedUnits SelectedUnits)
  (if (or (>= (Utilities|Array|Length (Variables|Unit|GetSelectedUnits)) 1) false)
    (Variables|Unit|SetIsUnitSelected true)))

(fn GetUnitHud
  (bind _selectableobjectsenum (Variables|HitResults|GetSelectableObjectsEnum))
  (bind _hitresult (Class|PlayerController|GetHitResultUnderCursorforObjects _selectableobjectsenum true))
  (bind _hitactor (Collision|BreakHitResult _hitresult))
  (if (!= _hitactor 0)
    (Default|CallDisplayHud _hitactor false)))

(fn StopPreviousCommand
  (bind _targetlocationdecal (Variables|Default|GetTargetLocationDecal))
  (Utilities|IsValid _targetlocationdecal
    (:Is%20Valid
      (Components|DestroyComponent _targetlocationdecal))
    (:Is%20Not%20Valid
      _))
  (AI|Navigation|StopMovement (Variables|Unit|GetAIController))
  (return))

(fn SetClickedActor
  (bind (_hitresult _returnvalue) (Game|Player|GetHitResultUnderCursorbyChannel "TraceTypeQuery1" false))
  (bind (_bblockinghit _binitialoverlap _time _distance _location _impactpoint _normal _impactnormal _physmat _hitactor) (Collision|BreakHitResult _hitresult))
  (if _returnvalue
    (Variables|Unit|SetTargetLocation (Utilities|FromGridtoWorld (Math|Conversions|ToVector(Float) (Utilities|ToGridLocattion (Math|Vector|MakeVector (.x _location) (.y _location) 0.0)))))
    (Variables|Unit|SetHitActor _hitactor)
    (return)))