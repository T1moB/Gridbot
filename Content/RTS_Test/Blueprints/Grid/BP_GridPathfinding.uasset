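; Grid pathfinding Blueprint that runs A* between two tile indices, with optional diagonal movement.
; FindPath keeps discovered tiles in cost-sorted parallel arrays, expands the cheapest, and rebuilds the path from previous-index links once the target is discovered.
; Neighbours must be walkable and within one tile height, and diagonal steps add a 0.5 penalty.
; It marks analyzed tiles on the Grid and signals data updates and clears.
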(event EventBeginPlay)

(event Collision|EventActorBeginOverlap
  (params (OtherActor :type Actor%20Object%20Reference)))

(event EventTick
  (params (DeltaSeconds :type Float%20%28single-precision%29)))

(fn ConstructionScript)

(fn GetValidTileNeighbours
  (params (Index :type Int%20Point%20Structure) (IncludeDiagonals :type Boolean))
  (LocalVariables|SetInputData (.Value (Utilities|Map|Find (Variables|/Game/RTS_Test/Blueprints/Grid/BP_Grid.BP_Grid_C|GetGridTiles (Variables|Default|GetGrid)) Index)))
  (bind _neighbours (Neighbour|GetTileNeighbours Index IncludeDiagonals))
  (for _array_element _neighbours
    (bind _output_get (LocalVariables|SetData (.Value (Utilities|Map|Find (Variables|/Game/RTS_Test/Blueprints/Grid/BP_Grid.BP_Grid_C|GetGridTiles (Variables|Default|GetGrid)) _array_element))))
    (if (CallFunction|IsWalkable (.Type (Utilities|Struct|BreakS_TileData _output_get)))
      (if (<= (Math|Float|Absolute(Float) (- (.z (.location (.transform (LocalVariables|GetInputData)))) (.z (.location (.transform (LocalVariables|GetData)))))) (.z (Variables|/Game/RTS_Test/Blueprints/Grid/BP_Grid.BP_Grid_C|GetTile%20Size (Variables|Default|GetGrid))))
        (Utilities|Array|Add (LocalVariables|GetNeigbours) (Utilities|Struct|MakeS_PathfindingData (.index (LocalVariables|GetData)) 1.0 -9999.0 -9999.0 Index)))))
  (return (LocalVariables|GetNeigbours)))

(fn GetTileNeighbours
  (params (Index :type Int%20Point%20Structure) (IncludeDiagonals :type Boolean))
  (bind _intpoint (Utilities|Struct|MakeIntPoint 1 0))
  (bind _intpoint_2 (Utilities|Struct|MakeIntPoint 0 1))
  (bind _intpoint_3 (Utilities|Struct|MakeIntPoint -1 0))
  (bind _intpoint_4 (Utilities|Struct|MakeIntPoint 0 -1))
  (bind _returnvalue (+ Index _intpoint))
  (bind _returnvalue_2 (+ Index _intpoint_2))
  (bind _returnvalue_3 (+ Index _intpoint_3))
  (bind _returnvalue_4 (+ Index _intpoint_4))
  (bind _array (Utilities|Array|MakeArray _returnvalue _returnvalue_2 _returnvalue_3 _returnvalue_4))
  (if IncludeDiagonals
    (LocalVariables|SetNeigbours _array)
    (Utilities|Array|AppendArray (LocalVariables|GetNeigbours) (Utilities|Array|MakeArray (+ Index (Utilities|Struct|MakeIntPoint 1 1)) (+ Index (Utilities|Struct|MakeIntPoint -1 1)) (+ Index (Utilities|Struct|MakeIntPoint -1 -1)) (+ Index (Utilities|Struct|MakeIntPoint 1 -1))))
    (return (LocalVariables|GetNeigbours))
    (else
      (return _array))))

(fn FindPath
  (params (Start :type Int%20Point%20Structure) (Target :type Int%20Point%20Structure) (Diagonals :type Boolean))
  (Variables|Default|SetStartIndex Start)
  (Variables|Default|SetTargetIndex Target)
  (Variables|Default|SetUseDiagonals Diagonals)
  (CallFunction|ClearGeneratedDAta)
  (bind _isvalid (CallFunction|IsInputValid))
  (if _isvalid
    (CallFunction|DiscoverTile (Utilities|Struct|MakeS_PathfindingData (Variables|Default|GetStartIndex) 1.0 -9999.0 (CallFunction|GetMinimumCostBetweenTiles (Variables|Default|GetStartIndex) (Variables|Default|GetTargetIndex) (Variables|Default|GetUseDiagonals)) "(X=-999,Y=-999)"))
    (while (> (Utilities|Array|Length (Variables|Default|GetDiscoverdIndexes)) 0)
      (bind _foundtarget (CallFunction|AnalyzeNextDiscoverTile))
      (if _foundtarget
        (bind _path (CallFunction|GeneratePath))
        (return _path)))
    (return (Utilities|Array|MakeArray ""))
    (else
      (return (Utilities|Array|MakeArray "")))))

(fn IsInputValid
  (bind _grid (Variables|Default|GetGrid))
  (return (Math|Boolean|ANDBoolean (!= (Variables|Default|GetStartIndex) (Variables|Default|GetTargetIndex)) (Default|IsTileWalkable _grid (Variables|Default|GetStartIndex)) (Default|IsTileWalkable _grid (Variables|Default|GetTargetIndex)))))

(fn DiscoverTile
  (params (TileData :type S%20Pathfinding%20Data%20Structure))
  (bind _index (Utilities|Struct|BreakS_PathfindingData TileData))
  (Utilities|Map|Add (Variables|Default|GetPathfindingData) _index TileData)
  (CallFunction|InsertTileinDiscoverd TileData)
  (Default|CallOnPathFindingDataUpdated _index))

(fn GetMinimumCostBetweenTiles
  (params (Index1 :type Int%20Point%20Structure) (Index2 :type Int%20Point%20Structure) (Diagonals :type Boolean))
  (bind _returnvalue (- Index1 Index2))
  (bind _returnvalue_2 (- Index1 Index2))
  (if Diagonals
    (return (Math|Conversions|ToFloat(Integer) (Math|Integer|Max(Integer) (Math|Integer|Absolute(Integer) (.x _returnvalue_2)) (Math|Integer|Absolute(Integer) (.y _returnvalue_2)))))
    (else
      (return (Math|Conversions|ToFloat(Integer) (+ (Math|Integer|Absolute(Integer) (.x _returnvalue)) (Math|Integer|Absolute(Integer) (.y _returnvalue))))))))

(fn AnalyzeNextDiscoverTile
  (bind _tilepathdata (CallFunction|PullCheapestfromDiscovered))
  (bind _output_get (Variables|Default|SetCurrentAnalyzedTile _tilepathdata))
  (Default|AddStatetoTile (Variables|Default|GetGrid) (Utilities|Struct|BreakS_PathfindingData _output_get) "NewEnumerator6")
  (bind _neighbours (Neighbour|GetValidTileNeighbours (Utilities|Struct|BreakS_PathfindingData _output_get) (Variables|Default|GetUseDiagonals)))
  (bind _output_get_2 (Variables|Default|SetCurrentNeighbours _neighbours))
  (while (> (Utilities|Array|Length _output_get_2) 0)
    (bind _istargettile (CallFunction|DiscoverNextNeighbour))
    (if _istargettile
      (return true)))
  (return false))

(fn GeneratePath
  (LocalVariables|SetCurrent (Variables|Default|GetTargetIndex))
  (while (!= (LocalVariables|GetCurrent) (Variables|Default|GetStartIndex))
    (Utilities|Array|Add (LocalVariables|GetInvertedPath) (LocalVariables|GetCurrent))
    (LocalVariables|SetCurrent (.PerviousIndex (Utilities|Struct|BreakS_PathfindingData (.Value (Utilities|Map|Find (Variables|Default|GetPathfindingData) (LocalVariables|GetCurrent)))))))
  (Utilities|Array|Reverse (LocalVariables|GetInvertedPath))
  (return (LocalVariables|GetInvertedPath)))

(fn PullCheapestfromDiscovered
  (LocalVariables|SetTileIndex (Utilities|Array|Get(acopy) (Variables|Default|GetDiscoverdIndexes)))
  (Utilities|Array|RemoveIndex (Variables|Default|GetDiscoverdTileCosts))
  (Utilities|Array|RemoveIndex (Variables|Default|GetDiscoverdIndexes))
  (Utilities|Array|Add (Variables|Default|GetAnalyzedIndexes) (LocalVariables|GetTileIndex))
  (return (.Value (Utilities|Map|Find (Variables|Default|GetPathfindingData) (LocalVariables|GetTileIndex)))))

(fn DiscoverNextNeighbour
  (Variables|Default|SetCurrentNeighbour (Utilities|Array|Get(acopy) (Variables|Default|GetCurrentNeighbours)))
  (Utilities|Array|RemoveIndex (Variables|Default|GetCurrentNeighbours))
  (if (not (Utilities|Array|ContainsItem (Variables|Default|GetAnalyzedIndexes) (Utilities|Struct|BreakS_PathfindingData (Variables|Default|GetCurrentNeighbour))))
    (LocalVariables|SetCostFromStart (CallFunction|CalculateCostfromStart (Variables|Default|GetCurrentAnalyzedTile) (Variables|Default|GetCurrentNeighbour)))
    (bind _output_get (LocalVariables|SetIndexInDiscoverd (Utilities|Array|FindItem (Variables|Default|GetDiscoverdIndexes) (Utilities|Struct|BreakS_PathfindingData (Variables|Default|GetCurrentNeighbour)))))
    (if (== _output_get -1) ; New Neighbour?
      _
      (else
        (bind _output_get_2 (Variables|Default|SetCurrentNeighbour (.Value (Utilities|Map|Find (Variables|Default|GetPathfindingData) (Utilities|Struct|BreakS_PathfindingData (Variables|Default|GetCurrentNeighbour))))))
        (if (< (LocalVariables|GetCostFromStart) (Utilities|Struct|BreakS_PathfindingData _output_get_2))
          (Utilities|Array|RemoveIndex (Variables|Default|GetDiscoverdIndexes) (LocalVariables|GetIndexInDiscoverd))
          (Utilities|Array|RemoveIndex (Variables|Default|GetDiscoverdTileCosts) (LocalVariables|GetIndexInDiscoverd))
          (else
            (return false)))))
    (CallFunction|DiscoverTile (Utilities|Struct|MakeS_PathfindingData (.Index (Utilities|Struct|BreakS_PathfindingData (Variables|Default|GetCurrentNeighbour))) (.CostToEnterTIle (Utilities|Struct|BreakS_PathfindingData (Variables|Default|GetCurrentNeighbour))) (LocalVariables|GetCostFromStart) (CallFunction|GetMinimumCostBetweenTiles (Utilities|Struct|BreakS_PathfindingData (Variables|Default|GetCurrentNeighbour)) (Variables|Default|GetTargetIndex) (Variables|Default|GetUseDiagonals)) (Utilities|Struct|BreakS_PathfindingData (Variables|Default|GetCurrentAnalyzedTile))))
    (if (Class|KismetMathLibrary|EqualIntPointIntPoint (Utilities|Struct|BreakS_PathfindingData (Variables|Default|GetCurrentNeighbour)) (Variables|Default|GetTargetIndex))
      (return true)
      (else
        (return false)))
    (else
      (return false))))

(fn InsertTileinDiscoverd
  (params (Data :type S%20Pathfinding%20Data%20Structure))
  (bind (_costfromstart _minimumcosttotarget) (Utilities|Struct|BreakS_PathfindingData Data))
  (bind _discoverdtilecosts (Variables|Default|GetDiscoverdTileCosts))
  (LocalVariables|SetSortingCost (+ _costfromstart _minimumcosttotarget))
  (if (== (Utilities|Array|Length (Variables|Default|GetDiscoverdTileCosts)) 0)
    (Utilities|Array|Add (Variables|Default|GetDiscoverdTileCosts) (LocalVariables|GetSortingCost) :!label _label)
    (Utilities|Array|Add (Variables|Default|GetDiscoverdIndexes) (Utilities|Struct|BreakS_PathfindingData Data))
    (elif (>= (LocalVariables|GetSortingCost) (Utilities|Array|Get(acopy) _discoverdtilecosts (Utilities|Array|LastIndex _discoverdtilecosts)))
      (goto _label)
      (else
        (bind (_array_element _array_index) (Utilities|Array|ForEachLoopwithBreak (Variables|Default|GetDiscoverdTileCosts) :!label _label_2)
          (:LoopBody
            (if (>= _array_element (LocalVariables|GetSortingCost))
              (Utilities|Array|Insert (Variables|Default|GetDiscoverdTileCosts) (LocalVariables|GetSortingCost) _array_index)
              (Utilities|Array|Insert (Variables|Default|GetDiscoverdIndexes) (Utilities|Struct|BreakS_PathfindingData Data) _array_index)
              (goto _label_2 Break))))))))

(fn ClearGeneratedDAta
  (bind _keys (Utilities|Map|Keys (Variables|Default|GetPathfindingData)))
  (for _array_element _keys
    (Default|RemoveStatefromTile (Variables|Default|GetGrid) _array_element "NewEnumerator5")
    (Default|RemoveStatefromTile (Variables|Default|GetGrid) _array_element "NewEnumerator6"))
  (Utilities|Map|Clear (Variables|Default|GetPathfindingData))
  (Utilities|Array|Clear (Variables|Default|GetDiscoverdTileCosts))
  (Utilities|Array|Clear (Variables|Default|GetAnalyzedIndexes))
  (Utilities|Array|Clear (Variables|Default|GetDiscoverdIndexes))
  (Default|CallOnPathfindingDataCleared))

(fn IsDiagonal
  (params (Index1 :type Int%20Point%20Structure) (Index2 :type Int%20Point%20Structure))
  (bind _neighbours (Neighbour|GetTileNeighbours Index1 false))
  (return (not (Utilities|Array|ContainsItem _neighbours Index2))))

(fn CalculateTileSortingCost
  (params (S_PathfindingData :type S%20Pathfinding%20Data%20Structure%20%28by%20ref%29))
  (bind (_costfromstart _minimumcosttotarget) (Utilities|Struct|BreakS_PathfindingData S_PathfindingData))
  (bind (_index _perviousindex) (Utilities|Struct|BreakS_PathfindingData S_PathfindingData))
  (return (Math|Float|Truncate (+ (* (+ _costfromstart _minimumcosttotarget) 2.0) (Math|Conversions|ToInteger(Boolean) (CallFunction|IsDiagonal _index _perviousindex))))))

(fn CalculateCostfromStart
  (params (S_PathfindingData :type S%20Pathfinding%20Data%20Structure%20%28by%20ref%29) (S_PathfindingData2 :type S%20Pathfinding%20Data%20Structure%20%28by%20ref%29))
  (return (+ (Utilities|Struct|BreakS_PathfindingData S_PathfindingData) (+ (Utilities|Struct|BreakS_PathfindingData S_PathfindingData2) (Math|Float|SelectFloat 0.5 0.0 (CallFunction|IsDiagonal (.index (Variables|Default|GetCurrentAnalyzedTile)) (.index (Variables|Default|GetCurrentNeighbour))))))))