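; BP_GridVisual is the actor that draws the visual layer of a tile grid, with tick disabled at BeginPlay.
; It caches a BP_GridMeshInst child actor, then updates each tile by removing its instance and re-adding it with transform and state if walkable.
; Destroying the visual clears those instances.
; Mesh initialization with a flat square mesh is disconnected, and ground offset and grid fill functions are empty stubs.
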(event EventBeginPlay
  (Actor|Tick|SetActorTickEnabled false))

(event Collision|EventActorBeginOverlap
  (params (OtherActor :type Actor%20Object%20Reference)))

(event EventTick
  (params (DeltaSeconds :type Float%20%28single-precision%29)))

(fn ConstructionScript)

(fn InitializeGridVisual
  (params (Grid :type BP%20Grid%20Object%20Reference))
  (Variables|Default|SetGrid Grid)
  (Variables|Default|SetGrid%20Mesh%20Inst (.AsBP%20Grid%20Mesh%20Inst (Utilities|Casting|CastToBP_GridMeshInst (Variables|/Script/Engine.ChildActorComponent|GetChildActor (Variables|Default|GetChildActor_GridMeshInst)))))
  (Transformation|SetActorLocation (Math|Vector|MakeVector 0.0 0.0 0.0) false false))

(fn SetOffsetfromGround
  (params (Offset :type Float%20%28double-precision%29)))

(fn DestroyGridVisual
  (bind _grid_mesh_inst (Variables|Default|GetGrid%20Mesh%20Inst))
  (Utilities|IsValid _grid_mesh_inst
    (:Is%20Valid
      (Default|ClearInstance _grid_mesh_inst))))

(fn UpdateTileVisual
  (params (Data :type S%20Tile%20Data%20Structure))
  (Default|RemoveInstance (Variables|Default|GetGrid%20Mesh%20Inst) (.index Data))
  (if (CallFunction|IsWalkable (.type Data))
    (Default|AddInstance (Variables|Default|GetGrid%20Mesh%20Inst) (.index Data) (.transform Data) (.state Data))))

(fn SetGridFilled
  (params (GridIndex :type Int%20Point%20Structure)))