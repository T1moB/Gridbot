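; RTS HUD that draws a drag-box marquee and selects ground units inside it.
; Input start, hold and release events track the box corners from the player controller's mouse position, with a new press clearing the previous selection.
; While dragging, DrawHUD renders the rectangle and gathers actors with GetActorsInSelectionRectangle.
; On release, non-hidden units get selection decals and flags, and the list is passed back to the controller.
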(event Custom|DrawMarquee
  (bind _clickedlocation (Variables|MarqueeVariables|GetClickedLocation))
  (bind _holdinglocation (Variables|MarqueeVariables|GetHoldingLocation))
  (bind _clickedlocation_2 (Variables|MarqueeVariables|GetClickedLocation))
  (bind _holdinglocation_2 (Variables|MarqueeVariables|GetHoldingLocation))
  (bind (_x _y) (Math|Vector2D|BreakVector2D _holdinglocation))
  (bind (_x_2 _y_2) (Math|Vector2D|BreakVector2D _clickedlocation_2))
  (bind _returnvalue (- _holdinglocation_2 _clickedlocation_2))
  (bind (_x_3 _y_3) (Math|Vector2D|BreakVector2D _clickedlocation))
  (bind (_x_4 _y_4) (Math|Vector2D|BreakVector2D _returnvalue))
  (HUD|DrawRect "(R=0,G=0,B=0,A=1)" _x_3 _y_3 0.0 0.0)
  (HUD|DrawRect "(R=0,G=0,B=0,A=1)" _x _y 0.0 0.0)
  (HUD|DrawRect "(R=0.203470,G=0.452119,B=0.700000,A=0.600000)" _x_2 _y_2 _x_4 _y_4))

(event EventBeginPlay
  (Variables|References|SetControllerRef (.AsRTS%20Player%20Controller%20BP (Utilities|Casting|CastToRTS_PlayerController_BP (Game|GetPlayerController 0)))))

(event EventOnInputStart
  (bind _controllerref (Variables|References|GetControllerRef))
  (bind (_locationx _locationy) (Game|Player|GetMousePosition _controllerref))
  (if (>= (Utilities|Array|Length (Variables|Units|GetSelectedUnits)) 1)
    (CallFunction|DeselectUnits)
    (Default|SetSelectedUnits (Variables|References|GetControllerRef) (Variables|Units|GetSelectedUnits)))
  (bind _output_get (Variables|MarqueeVariables|SetClickedLocation (Math|Vector2D|MakeVector2D _locationx _locationy)))
  (Variables|MarqueeVariables|SetHoldingLocation _output_get)
  (Variables|Bool|SetIsDrawing true))

(event EventOnInputRelease
  (params (HoldTime :type Float%20%28double-precision%29))
  (Variables|Bool|SetIsDrawing false)
  (CallFunction|SetUnitsandVehicles)
  (Default|SetSelectedUnits (Variables|References|GetControllerRef) (Variables|Units|GetSelectedUnits)))

(event EventDrawHUD
  (params (SizeX :type Integer) (SizeY :type Integer))
  (if (Variables|Bool|GetIsDrawing)
    (Utilities|FlowControl|Sequence
      (:then_0
        (CallFunction|DrawMarquee))
      (:then_1
        (Variables|Units|SetUnitsInSelectionArea (Class|HUD|GetActorsinSelectionRectangle "/Game/RTS_Test/Blueprints/Units/RTS_GroundUnitMaster.RTS_GroundUnitMaster_C" (Variables|MarqueeVariables|GetClickedLocation) (Variables|MarqueeVariables|GetHoldingLocation) true false))))))

(event EventOnInputHold
  (bind _controllerref (Variables|References|GetControllerRef))
  (bind (_locationx _locationy) (Game|Player|GetMousePosition _controllerref))
  (Variables|MarqueeVariables|SetHoldingLocation (Math|Vector2D|MakeVector2D _locationx _locationy)))

(fn ConstructionScript)

(fn DeselectUnits
  (for _array_element (Variables|Units|GetSelectedUnits)
    (Default|SetDeselectedDecal _array_element)
    (Variables|/Game/RTS_Test/Blueprints/Units/RTS_GroundUnitMaster.RTS_GroundUnitMaster_C|SetIsSelected _array_element false)
    (Variables|/Game/RTS_Test/Blueprints/GameSettings/RTS_PlayerController_BP.RTS_PlayerController_BP_C|SetIsUnitSelected (Variables|References|GetControllerRef) false))
  (Utilities|Array|Clear (Variables|Units|GetSelectedUnits)))

(fn SetUnitsandVehicles
  (for _array_element (Variables|Units|GetUnitsInSelectionArea)
    (if (Utilities|ClassIsChildOf (Utilities|GetClass _array_element) "/Game/RTS_Test/Blueprints/Units/RTS_GroundUnitMaster.RTS_GroundUnitMaster_C")
      (bind _asrts_ground_unit_master (Utilities|Casting|CastToRTS_GroundUnitMaster _array_element))
      (if (not (Variables|/Game/RTS_Test/Blueprints/Units/RTS_GroundUnitMaster.RTS_GroundUnitMaster_C|GetIsHidden _asrts_ground_unit_master))
        (Utilities|Array|AddUnique (Variables|Units|GetSelectedUnits) _asrts_ground_unit_master))))
  (Utilities|FlowControl|Sequence
    (:then_0
      (for _array_element_2 (Variables|Units|GetSelectedUnits)
        (Default|SetSelectedDecal _array_element_2)
        (Variables|/Game/RTS_Test/Blueprints/Units/RTS_GroundUnitMaster.RTS_GroundUnitMaster_C|SetIsSelected _array_element_2 true)))))