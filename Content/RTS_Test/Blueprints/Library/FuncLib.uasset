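; Blueprint function library for the RTS_Test game, providing game clock math and a mouse-to-world position lookup.
; SetGameTime divides DeltaTime by GameSpeed, adds the initial time and splits the result by a 24-hour cycle into time of day and day count.
; GetMousePosInWorld deprojects the cursor, line traces along that ray up to SightDistance and returns the hit location when the hit-actor check passes.
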(fn SetGameTime
  (params (DeltaTime :type Float%20%28double-precision%29) (GameSpeed :type Float%20%28double-precision%29) (InitialGameTime :type Float%20%28double-precision%29))
  (bind _returnvalue (/ DeltaTime GameSpeed))
  (bind _returnvalue_2 (+ _returnvalue InitialGameTime))
  (bind (_remainder _returnvalue_3) (Math|Float|Division(WholeandRemainder) _returnvalue_2 24.0))
  (return _remainder _returnvalue_3))

(fn GetMousePosinWorld
  (params (Controller :type RTS%20Player%20Controller%20BP%20Object%20Reference) (SightDistance :type Float%20%28double-precision%29))
  (bind (_worldlocation _worlddirection) (Game|Player|ConvertMouseLocationToWorldSpace Controller))
  (bind _outhit (Collision|LineTraceByChannel 0 _worldlocation (+ _worldlocation (* _worlddirection SightDistance)) "TraceTypeQuery3" false 0 "None"))
  (if (!= (.HitActor (Collision|BreakHitResult _outhit)) 0)
    (return (.Location (Collision|BreakHitResult _outhit)))))