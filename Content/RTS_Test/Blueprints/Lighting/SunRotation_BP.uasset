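; Sun rotation Blueprint that drives the sun and sky from the game's clock.
; Caches the RTS game state at BeginPlay, then each tick converts its GameTime into a sun pitch of about 15 degrees per unit, offset by 90.
; After rotating the referenced sun actor, it calls UpdateSunDirection on the sky sphere so the sky follows.
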(event EventBeginPlay
  (Variables|Refrences|SetGameStateRef (.AsRTS%20Game%20State%20Base%20BP (Utilities|Casting|CastToRTS_GameStateBase_BP (Game|GetGameState)))))

(event EventTick
  (params (DeltaSeconds :type Float%20%28single-precision%29))
  (Transformation|SetActorRotation (Variables|Refrences|GetSunRef) (Math|Rotator|MakeRotator 0.0 (+ (* (* (Variables|/Game/RTS_Test/Blueprints/GameSettings/RTS_GameStateBase_BP.RTS_GameStateBase_BP_C|GetGameTime (Variables|Refrences|GetGameStateRef)) 3.6e+03) 0.004167) 9e+01) 0.0))
  (Default|UpdateSunDirection (Variables|Refrences|GetSkySphereRef)))

(fn ConstructionScript)