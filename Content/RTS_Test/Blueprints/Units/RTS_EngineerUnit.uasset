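; RTS Engineer unit Blueprint, a child unit class that identifies itself through a UnitType enum value.
; The construction script runs the parent logic, sets that type and attaches a ToolBox component to the "ToolBox" socket on the mesh.
; BeginPlay calls the parent and reapplies the type only when the unit is not flagged as spawned in.
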(event EventBeginPlay
  (|CallParentFunction)
  (if (not (Variables|Default|GetIsSpawnedIn))
    (Variables|Default|SetUnitType "NewEnumerator1")))

(event Collision|EventActorBeginOverlap
  (params (OtherActor :type Actor%20Object%20Reference)))

(event EventTick
  (params (DeltaSeconds :type Float%20%28single-precision%29))
  (|CallParentFunction DeltaSeconds) ; This node is disabled and will not be called.\nDrag off pins to build functionality.
)

(fn ConstructionScript
  (|CallParentFunction)
  (Variables|Default|SetUnitType "NewEnumerator1")
  (Transformation|AttachComponentToComponent (Variables|Default|GetToolBox) (Variables|Character|GetMesh) "ToolBox" "KeepRelative" "KeepRelative" "KeepRelative" true))