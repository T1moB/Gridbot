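; Infantry unit Blueprint for an RTS that carries a socketed rifle and fights an assigned target unit.
; Attacks start on a prepare event or when the target overlaps DamageEntry, running DoDamage on a looping timer.
; Each tick of that timer checks a frontal yaw cone, turning toward the target if needed, otherwise rolling a hit chance.
; Hits deal randomised base damage, scaled by a random bonus while support is active.
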(event OnComponentBeginOverlap(DamageEntry)
  (params (OverlappedComponent :type Primitive%20Component%20Object%20Reference) (OtherActor :type Actor%20Object%20Reference) (OtherComp :type Primitive%20Component%20Object%20Reference) (OtherBodyIndex :type Integer) (bFromSweep :type Boolean) (SweepResult :type Hit%20Result%20Structure%20%28by%20ref%29))
  (if (== OtherActor (Variables|Default|GetTargetUnit))
    (CallFunction|Attack)))

(event Custom|DoDamage
  (if (CallFunction|GetTargetRotation)
    (Utilities|CheckifHit
      (:Hit
        (bind _damage (CallFunction|SetDamage))
        (Default|ReduceHealth (Variables|Default|GetTargetUnit) _damage)
        (Utilities|IsValid (Variables|Default|GetTargetUnit)
          (:Is%20Not%20Valid
            (Utilities|Time|SetTimerbyFunctionName 0 "DoDamage" 0.0)))))
    (else
      (Utilities|LooktoTarget))))

(event EventBeginPlay
  (|CallParentFunction)
  (if (not (Variables|Default|GetIsSpawnedIn))
    (Variables|Default|SetUnitType "NewEnumerator0")))

(event Collision|EventActorBeginOverlap
  (params (OtherActor :type Actor%20Object%20Reference)))

(event EventTick
  (params (DeltaSeconds :type Float%20%28single-precision%29))
  (|CallParentFunction DeltaSeconds) ; This node is disabled and will not be called.\nDrag off pins to build functionality.
)

(event EventAttack
  (if (!= (Variables|Default|GetTargetUnit) self)
    (Utilities|Time|SetTimerbyFunctionName 0 "DoDamage" 1.0 true)))

(event EventStartSupport
  (Variables|Default|SetSupportDamageModifier (Math|Random|RandomFloatinRange 1.0 1.25)))

(event EventEndSupport
  (Variables|Default|SetSupportDamageModifier 1.0))

(event EventPreparetoAttack
  (if (CallFunction|GetTargetRotation)
    (CallFunction|Attack)
    (else
      (Utilities|LooktoTarget))))

(fn ConstructionScript
  (|CallParentFunction)
  (Variables|Default|SetUnitType "NewEnumerator0")
  (Transformation|AttachComponentToComponent (Variables|Default|GetRifle) (Variables|Character|GetMesh) "Weapon" "KeepRelative" "KeepRelative" "KeepRelative" true))

(fn SetDamage
  (Variables|Default|SetDamageModifier (Math|Random|RandomFloatinRange 0.25 1.5))
  (bind _output_get (Variables|Default|SetDamage (* (Variables|Default|GetBaseDamage) (Variables|Default|GetDamageModifier) (Variables|Default|GetSupportDamageModifier))))
  (return _output_get))

(fn GetTargetRotation
  (return (Math|Float|InRange(Float) (.yaw (Math|Rotator|Delta(Rotator) (Math|Rotator|FindLookatRotation (Transformation|GetActorLocation) (Transformation|GetActorLocation (Variables|Default|GetTargetUnit))) (Transformation|GetActorRotation))) -45.0 45.0)))