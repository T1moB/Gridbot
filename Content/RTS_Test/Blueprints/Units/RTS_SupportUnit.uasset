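; RTS support unit that repairs its target and toggles a support state on other ground units within its SupportEntry volume.
; Overlapping the assigned TargetUnit starts a looping RepairUnit timer, restoring health before armor in increments from SetGameTime using GameSpeed, then clamping to maximums and releasing the target.
; Other overlapping RTS_GroundUnitMaster units receive StartSupport, with only the latest stored in UnitToSupport for EndSupport on exit.
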(event OnComponentBeginOverlap(SupportEntry)
  (params (OverlappedComponent :type Primitive%20Component%20Object%20Reference) (OtherActor :type Actor%20Object%20Reference) (OtherComp :type Primitive%20Component%20Object%20Reference) (OtherBodyIndex :type Integer) (bFromSweep :type Boolean) (SweepResult :type Hit%20Result%20Structure%20%28by%20ref%29))
  (bind _targetunit (Variables|Default|GetTargetUnit))
  (if (and (== OtherActor _targetunit) (Utilities|IsValid _targetunit))
    (Variables|Default|SetIsAtTarget true)
    (CallFunction|HealUnit)
    (elif (and (Utilities|ClassIsChildOf (Utilities|GetClass OtherActor) "/Game/RTS_Test/Blueprints/Units/RTS_GroundUnitMaster.RTS_GroundUnitMaster_C") (!= OtherActor self))
      (Variables|Default|SetUnitToSupport (.AsRTS%20Ground%20Unit%20Master (Utilities|Casting|CastToRTS_GroundUnitMaster OtherActor)))
      (Default|StartSupport (Variables|Default|GetUnitToSupport)))))

(event OnComponentEndOverlap(SupportEntry)
  (params (OverlappedComponent :type Primitive%20Component%20Object%20Reference) (OtherActor :type Actor%20Object%20Reference) (OtherComp :type Primitive%20Component%20Object%20Reference) (OtherBodyIndex :type Integer))
  (if (== OtherActor (Variables|Default|GetTargetUnit))
    (Variables|Default|SetIsAtTarget false)
    (Variables|Default|SetTargetUnit 0)
    (elif (== OtherActor (Variables|Default|GetUnitToSupport))
      (Default|EndSupport (Variables|Default|GetUnitToSupport))
      (Variables|Default|SetUnitToSupport 0))))

(event EventBeginPlay
  (|CallParentFunction)
  (if (not (Variables|Default|GetIsSpawnedIn))
    (Variables|Default|SetUnitType "NewEnumerator3")))

(event Collision|EventActorBeginOverlap
  (params (OtherActor :type Actor%20Object%20Reference)))

(event EventTick
  (params (DeltaSeconds :type Float%20%28single-precision%29))
  (|CallParentFunction DeltaSeconds) ; This node is disabled and will not be called.\nDrag off pins to build functionality.
)

(event EventHealUnit
  (if (!= (Variables|Default|GetTargetUnit) self)
    (if (or (CallFunction|CheckTargetHealth) (CallFunction|CheckTargetArmor))
      (Utilities|Time|SetTimerbyFunctionName 0 "RepairUnit" 0.01 true))))

(fn ConstructionScript
  (|CallParentFunction)
  (Variables|Default|SetUnitType "NewEnumerator3"))

(fn CheckTargetHealth
  (bind _targetunit (Variables|Default|GetTargetUnit))
  (Utilities|IsValid _targetunit
    (:Is%20Valid
      (return (< (Variables|/Game/RTS_Test/Blueprints/Units/RTS_GroundUnitMaster.RTS_GroundUnitMaster_C|GetCurrentHealth _targetunit) (Variables|/Game/RTS_Test/Blueprints/Units/RTS_GroundUnitMaster.RTS_GroundUnitMaster_C|GetMaxHealth _targetunit))))))

(fn CheckTargetArmor
  (bind _targetunit (Variables|Default|GetTargetUnit))
  (Utilities|IsValid _targetunit
    (:Is%20Valid
      (return (< (Variables|/Game/RTS_Test/Blueprints/Units/RTS_GroundUnitMaster.RTS_GroundUnitMaster_C|GetCurrentArmor _targetunit) (Variables|/Game/RTS_Test/Blueprints/Units/RTS_GroundUnitMaster.RTS_GroundUnitMaster_C|GetMaxArmor _targetunit))))))

(fn RepairUnit
  (if (Variables|Default|GetIsAtTarget)
    (if (CallFunction|CheckTargetHealth)
      (bind _output_get (Variables|Default|SetRepairTime (.GameTime (CallFunction|SetGameTime (Variables|Default|GetDeltaTime) (Variables|Default|GetGameSpeed) (Variables|Default|GetRepairTime)))))
      (Variables|/Game/RTS_Test/Blueprints/Units/RTS_GroundUnitMaster.RTS_GroundUnitMaster_C|SetCurrentHealth (Variables|Default|GetTargetUnit) (+ (/ (* _output_get 6e+01) 1e+02) (Variables|/Game/RTS_Test/Blueprints/Units/RTS_GroundUnitMaster.RTS_GroundUnitMaster_C|GetCurrentHealth (Variables|Default|GetTargetUnit))))
      (Default|UpdateUnitHealthBar (Variables|Default|GetTargetUnit))
      (Variables|Default|SetRepairTime 0.01)
      (return)
      (elif (CallFunction|CheckTargetArmor)
        (bind _output_get_2 (Variables|Default|SetRepairTime (.GameTime (CallFunction|SetGameTime (Variables|Default|GetDeltaTime) (Variables|Default|GetGameSpeed) (Variables|Default|GetRepairTime)))))
        (Variables|/Game/RTS_Test/Blueprints/Units/RTS_GroundUnitMaster.RTS_GroundUnitMaster_C|SetCurrentArmor (Variables|Default|GetTargetUnit) (+ (/ (* _output_get_2 6e+01) 1e+02) (Variables|/Game/RTS_Test/Blueprints/Units/RTS_GroundUnitMaster.RTS_GroundUnitMaster_C|GetCurrentArmor (Variables|Default|GetTargetUnit))))
        (Default|UpdateUnitArmorBar (Variables|Default|GetTargetUnit))
        (Variables|Default|SetRepairTime 0.01)
        (return)
        (else
          (Variables|Default|SetRepairTime 0.0)
          (Variables|/Game/RTS_Test/Blueprints/Units/RTS_GroundUnitMaster.RTS_GroundUnitMaster_C|SetCurrentHealth (Variables|Default|GetTargetUnit) (Variables|/Game/RTS_Test/Blueprints/Units/RTS_GroundUnitMaster.RTS_GroundUnitMaster_C|GetMaxHealth (Variables|Default|GetTargetUnit)))
          (Variables|/Game/RTS_Test/Blueprints/Units/RTS_GroundUnitMaster.RTS_GroundUnitMaster_C|SetCurrentArmor (Variables|Default|GetTargetUnit) (Variables|/Game/RTS_Test/Blueprints/Units/RTS_GroundUnitMaster.RTS_GroundUnitMaster_C|GetMaxArmor (Variables|Default|GetTargetUnit)))
          (Utilities|Time|SetTimerbyFunctionName 0 "RepairUnit" 0.0)
          (Variables|Default|SetIsAtTarget false)
          (Variables|Default|SetTargetUnit 0)
          (return))))))